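; Side-scrolling Paper2D character, apparently the player, that moves along world X from the Move_right input axis.
; Each Tick swaps the sprite flipbook between Move_right and Stay based on whether velocity is non-zero.
; Tick also sets control rotation from the sign of X velocity, using -180 or 180 roll with zero yaw, which are equivalent orientations.
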(event `self.ReceiveTick`
  (params (DeltaSeconds :type "Float (single-precision)"))
  (`self.Animation`)
  (`self.rotation`))

(event `InputAxis|Move_right`
  (params (AxisValue :type "Float (single-precision)"))
  (`self.AddMovementInput` (1.0 0.0 0.0) AxisValue))

(event `Animation`
  (`PaperFlipbookComponent.SetFlipbook` (`self.Sprite`) (select `bool` (> (`KismetMathLibrary.VSize` (`MovementComponent.Velocity` (`self.CharacterMovement`))) 0.0) :`false` "/Game/character/stay.stay" :`true` "/Game/character/move_right.move_right" :!type "PaperFlipbook Object Reference")))

(event `rotation`
  (`/Engine/EditorBlueprintResources/StandardMacros.IsValid` (`self.GetController`)
    (:`Is Valid`
      (`/Engine/EditorBlueprintResources/StandardMacros.CompareFloat` (.x (`MovementComponent.Velocity` (`self.CharacterMovement`)))
        (:`>`
          (`Controller.SetControlRotation` (`self.GetController`) (`KismetMathLibrary.MakeRotator` -180.0 0.0 0.0)))
        (:`<`
          (`Controller.SetControlRotation` (`self.GetController`) (`KismetMathLibrary.MakeRotator` 180.0 0.0 0.0)))))))

(fn `UserConstructionScript`)